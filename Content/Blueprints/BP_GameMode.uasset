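; Game mode for a runner game that drives the flow from main menu through HUD to game-over screen.
; Play notifies the runner character and shows the HUD; retry reloads TestMap.
; Tick gradually raises the player's walk speed to a cap and updates the score text via CalculatePlayerScore.
; Player destruction and obstacle collision share a DoOnce that stops the game and shows the game-over screen.
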(event `self.ReceiveBeginPlay`
  (set `self.bGameRunning` true)
  (add `self.OnDestroyed` (`GameplayStatics.GetPlayerCharacter` 0) (delegate `NotifyPlayerDestroyed`))
  (bind _returnvalue (`|CreateWidget` "/Game/UI/WBP_MainMenu.WBP_MainMenu_C" (`GameplayStatics.GetPlayerController` 0)))
  (bind _output_get (set `self.MainMenu` _returnvalue))
  (`UserWidget.AddToViewport` _output_get 0)
  (add `Button.OnClicked` (`/Game/UI/WBP_MainMenu.PlayButton` _output_get) (delegate `ButtonPlayClicked`)))

(event `ButtonPlayClicked`
  (`Widget.RemoveFromParent` (`self.MainMenu`))
  (bind _asbp_runner_character (cast `/Game/Blueprints/BP_RunnerCharacter` (`GameplayStatics.GetPlayerCharacter` 0)))
  (`RunnerCharacter.NotifyGameStarted` _asbp_runner_character)
  (bind _returnvalue (`|CreateWidget` "/Game/UI/WBP_HUD.WBP_HUD_C" (`GameplayStatics.GetPlayerController` 0)))
  (bind _output_get (set `self.HUD` _returnvalue))
  (`UserWidget.AddToViewport` _output_get 0))

(event `NotifyPlayerDestroyed` :!signature `self.OnDestroyed`
  (params (DestroyedActor :type "Actor Object Reference"))
  (`/Engine/EditorBlueprintResources/StandardMacros.DoOnce` false :!label _label
    (:`Completed`
      (set `self.bGameRunning` false)
      (bind _returnvalue (`|CreateWidget` "/Game/UI/WBP_GameOverScreen.WBP_GameOverScreen_C" (`GameplayStatics.GetPlayerController` 0)))
      (bind _output_get (set `self.GameOverScreen` _returnvalue))
      (`UserWidget.AddToViewport` _output_get 0)
      (add `Button.OnClicked` (`/Game/UI/WBP_GameOverScreen.ButtonRetry` _output_get) (delegate `ButonReplayClicked`)))))

(event `self.NotifyPlayerObstacleCollision`
  (bind _asbp_runner_character (cast `/Game/Blueprints/BP_RunnerCharacter` (`GameplayStatics.GetPlayerCharacter` 0)))
  (`RunnerCharacter.NotifyObstacleCollision` _asbp_runner_character)
  (goto _label))

(event `ButonReplayClicked`
  (`Widget.RemoveFromParent` (`self.GameOverScreen`))
  (`Widget.RemoveFromParent` (`self.HUD`))
  (`GameplayStatics.OpenLevel` "TestMap"))

(event `self.ReceiveTick`
  (params (DeltaSeconds :type "Float (single-precision)"))
  (bind _hud (`self.HUD`))
  (if (`self.bGameRunning`)
    (`self.UpdatePlayerMovementSpeed` DeltaSeconds)
    (`/Engine/EditorBlueprintResources/StandardMacros.IsValid` _hud
      (:`Is Valid`
        (`/Game/UI/WBP_HUD.SetScoreText` _hud (`self.CalculatePlayerScore`))))))

(fn `UpdatePlayerMovementSpeed`
  (params (B :type "Float (double-precision)"))
  (bind _characterspeed (`self.CharacterSpeed`))
  (if (< _characterspeed 1000.0)
    (set `self.CharacterSpeed` (+ _characterspeed (* 10.0 B)))
    (bind _asbp_runner_character (cast `/Game/Blueprints/BP_RunnerCharacter` (`GameplayStatics.GetPlayerCharacter` 0)))
    (set `CharacterMovementComponent.MaxWalkSpeed` (`self.CharacterSpeed`) (`Character.CharacterMovement` _asbp_runner_character))))

(fn `UserConstructionScript`)